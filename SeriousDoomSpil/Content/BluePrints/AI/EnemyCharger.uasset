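; EnemyCharger is a suicide-attack enemy that starts in a configured Roam, Patrol or Chase state.
; Roam moves to random navigable points and Patrol loops between two target points, while PawnSensing triggers a chase ending in damage, explosion and self-destruction.
; Player death disables sensing and re-enters the configured state.
; AnyDamage reduces health, and a Tick check destroys the enemy at zero, awarding the player points.
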(event OnSeePawn(PawnSensing)
  (params (Pawn :type Pawn%20Object%20Reference))
  ;[1 1 1] Chase state enabler
  (bind _asthird_person_character (Utilities|Casting|CastToThirdPersonCharacter Pawn))
  (CallFunction|ChasePlayer _asthird_person_character))

(event Custom|Patrol
  ;[1 1 1] Patrol State
  (AI|AIMoveTo self "0, 0, 0" (Variables|Default|GetTargetPoint1) 5.0 false
    (:OnSuccess
      (Utilities|FlowControl|Delay 0.5)
      (AI|AIMoveTo self "0, 0, 0" (Variables|Default|GetTargetPoint2) 5.0 false
        (:OnSuccess
          (Utilities|FlowControl|Delay 0.5)
          (CallFunction|Patrol))))))

(event Custom|ResetAI
  ;[1 1 1] Reset to former AIState
  (Class|PawnSensingComponent|SetSensingUpdatesEnabled (Variables|Default|GetPawnSensing) false)
  (switch Utilities|FlowControl|Switch|SwitchonEAIState (Variables|Default|GetAIState)
    (:NewEnumerator1
      (CallFunction|Roam))
    (:NewEnumerator2
      (CallFunction|ChasePlayer))
    (:NewEnumerator3
      (CallFunction|Patrol))))

(event Custom|ChasePlayer
  (params (PlayerToChase :type Pawn%20Object%20Reference))
  (bind _returnvalue (Transformation|GetActorLocation))
  ;[1 1 1] Chase state
  (if (Variables|/Script/AIModule.PawnSensingComponent|GetbEnableSensingUpdates (Variables|Default|GetPawnSensing))
    (AI|AIMoveTo self "0, 0, 0" PlayerToChase 5.0 false
      (:OnSuccess
        (Game|Damage|ApplyDamage PlayerToChase (Variables|Default|GetDamage) 0 0)
        (Effects|SpawnEmitteratLocation "/Game/InfinityBladeEffects/Effects/FX_Mobile/combat/P_Impact_Golem_Death_Fire.P_Impact_Golem_Death_Fire" _returnvalue "0, 0, 0" "2.000000,2.000000,2.000000")
        (Audio|PlaySoundatLocation "/Game/StarterContent/Audio/Explosion01.Explosion01" _returnvalue)
        (Actor|DestroyActor)))))

(event Custom|Roam
  ;[1 1 1] Roam State
  (AI|AIMoveTo self (.RandomLocation (Class|NavigationSystem|GetRandomPointinNavigableRadius (Transformation|GetActorLocation) 5e+02)) 0 5.0 false
    (:OnSuccess
      (Utilities|FlowControl|Delay 0.5)
      (CallFunction|Roam))))

(event EventBeginPlay
  ;[1 1 1] AI Startup (state is set in EnemyCharger -> Default
  (bind _asthird_person_character (Utilities|Casting|CastToThirdPersonCharacter (Game|GetPlayerCharacter 0)))
  (EventDispatchers|BindEventtoPlayerDied _asthird_person_character (delegate Custom|ResetAI))
  (switch Utilities|FlowControl|Switch|SwitchonEAIState (Variables|Default|GetAIState)
    (:NewEnumerator1
      (CallFunction|Roam))
    (:NewEnumerator2
      (CallFunction|ChasePlayer))
    (:NewEnumerator3
      (CallFunction|Patrol))))

(event EventTick
  (params (DeltaSeconds :type Float%20%28single-precision%29))
  ;[1 1 1] Take damage
  ;;[1 1 1] Healthcheck (if health <= 0 then DestroyActor)
  (if (<= (Variables|Default|GetCurrentHealth) 0.0)
    (Actor|DestroyActor)
    (bind _asthird_person_character (Utilities|Casting|CastToThirdPersonCharacter (Game|GetPlayerCharacter 0)))
    (Variables|/Game/ThirdPersonBP/Blueprints/ThirdPersonCharacter.ThirdPersonCharacter_C|SetPoints _asthird_person_character (+ (Variables|/Game/ThirdPersonBP/Blueprints/ThirdPersonCharacter.ThirdPersonCharacter_C|GetPoints _asthird_person_character) 5.0))))

(event Game|Damage|EventAnyDamage
  (params (Damage :type Float%20%28single-precision%29) (DamageType :type Damage%20Type%20Object%20Reference) (InstigatedBy :type Controller%20Object%20Reference) (DamageCauser :type Actor%20Object%20Reference))
  ;[1 1 1] Take damage
  (Variables|Default|SetCurrentHealth (- (Variables|Default|GetCurrentHealth) Damage)))

(fn ConstructionScript)