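; EnemyShooter is an AI enemy that roams or patrols and shoots at the player on sight.
; AIState picks looping AIMoveTo behavior: random navmesh points or two target points.
; PawnSensing turns it toward the player and fires impulse-launched projectiles behind a delay-based cooldown.
; Damage lowers health, Tick destroys it at zero and awards points, and player death disables sensing and restarts movement.
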(event OnSeePawn(PawnSensing)
  (params (Pawn :type Pawn%20Object%20Reference))
  ;[1 1 1] Rotate and shoot
  (bind _asthird_person_character (Utilities|Casting|CastToThirdPersonCharacter Pawn))
  (Utilities|FlowControl|Sequence
    (:then_0
      (Transformation|SetActorRotation (Math|Rotator|FindLookatRotation (Transformation|GetActorLocation) (Transformation|GetActorLocation _asthird_person_character))))
    (:then_1
      (if (Variables|Default|GetSpawnProjectile)
        (bind _returnvalue (Game|SpawnActorfromClass "/Game/BluePrints/EnemyProjectile.EnemyProjectile_C" (Transformation|GetWorldTransform (Variables|Default|GetProjectileSpawnLocation)) "Undefined" 0 0))
        (Physics|AddImpulse (Variables|/Game/BluePrints/EnemyProjectile.EnemyProjectile_C|GetStaticMesh _returnvalue) (* (Math|Vector|GetForwardVector (Variables|Default|GetSphere)) (Variables|Default|GetShootForce)) "None" false)
        (Variables|Default|SetSpawnProjectile false)
        (Utilities|FlowControl|Delay 2.0)
        (Variables|Default|SetSpawnProjectile true)))))

(event Custom|Patrol
  ;[1 1 1] Patrol State
  (AI|AIMoveTo self "0, 0, 0" (Variables|Default|GetTargetPoint1) 5.0 false
    (:OnSuccess
      (Utilities|FlowControl|Delay 0.5)
      (AI|AIMoveTo self "0, 0, 0" (Variables|Default|GetTargetPoint2) 5.0 false
        (:OnSuccess
          (Utilities|FlowControl|Delay 0.5)
          (CallFunction|Patrol))))))

(event Custom|ResetAI
  ;[1 1 1] Reset to former AIState if player dead
  (Class|PawnSensingComponent|SetSensingUpdatesEnabled (Variables|Default|GetPawnSensing) false)
  (switch Utilities|FlowControl|Switch|SwitchonEAIState (Variables|Default|GetAIState)
    (:NewEnumerator1
      (CallFunction|Roam))
    (:NewEnumerator3
      (CallFunction|Patrol))))

(event Custom|Roam
  ;[1 1 1] Roam State
  (AI|AIMoveTo self (.RandomLocation (Class|NavigationSystem|GetRandomPointinNavigableRadius (Transformation|GetActorLocation) 5e+02)) 0 5.0 false
    (:OnSuccess
      (Utilities|FlowControl|Delay 0.5)
      (CallFunction|Roam))))

(event EventBeginPlay
  ;[1 1 1] AI Startup (state is set in EnemyShooter -> Default)
  (bind _asthird_person_character (Utilities|Casting|CastToThirdPersonCharacter (Game|GetPlayerCharacter 0)))
  (EventDispatchers|BindEventtoPlayerDied _asthird_person_character (delegate Custom|ResetAI))
  (switch Utilities|FlowControl|Switch|SwitchonEAIState (Variables|Default|GetAIState)
    (:NewEnumerator1
      (CallFunction|Roam))
    (:NewEnumerator3
      (CallFunction|Patrol))))

(event EventTick
  (params (DeltaSeconds :type Float%20%28single-precision%29))
  ;[1 1 1] Take damage
  ;;[1 1 1] Healthcheck (if health <= 0 then DestroyActor)
  (if (<= (Variables|Default|GetCurrentHealth) 0.0)
    (Actor|DestroyActor)
    (bind _asthird_person_character (Utilities|Casting|CastToThirdPersonCharacter (Game|GetPlayerCharacter 0)))
    (Variables|/Game/ThirdPersonBP/Blueprints/ThirdPersonCharacter.ThirdPersonCharacter_C|SetPoints _asthird_person_character (+ (Variables|/Game/ThirdPersonBP/Blueprints/ThirdPersonCharacter.ThirdPersonCharacter_C|GetPoints _asthird_person_character) 5.0))))

(event Game|Damage|EventAnyDamage
  (params (Damage :type Float%20%28single-precision%29) (DamageType :type Damage%20Type%20Object%20Reference) (InstigatedBy :type Controller%20Object%20Reference) (DamageCauser :type Actor%20Object%20Reference))
  ;[1 1 1] Take damage
  (Variables|Default|SetCurrentHealth (- (Variables|Default|GetCurrentHealth) Damage)))

(fn ConstructionScript)